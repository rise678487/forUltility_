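; Test actor for anchor points that visualizes the path and distance to its NearestAnchorPoint.
; After a short delay on BeginPlay, it sphere-traces toward that point, printing each hit actor and drawing a distance-sized debug sphere around itself.
; FindNearestPoint scans an anchor array for the closest, stores it and returns a look-at rotation.
; Its calls, which would rotate the Arrow, are disconnected, so live logic never updates NearestAnchorPoint.
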(event `self.ReceiveBeginPlay`
  (bind _returnvalue (`self.K2_GetActorLocation`))
  (bind _returnvalue_2 (`self.K2_GetActorLocation` (`self.NearestAnchorPoint`)))
  (`KismetSystemLibrary.Delay` 2.0)
  (bind _outhits (`KismetSystemLibrary.SphereTraceMulti` :`Start` _returnvalue :`End` _returnvalue_2 :`Radius` 1.0 :`TraceChannel` "TraceTypeQuery1" :`DrawDebugType` "ForDuration" :`DrawTime` 10.0))
  (for _array_element _outhits
    (`KismetSystemLibrary.PrintString` (`KismetSystemLibrary.GetDisplayName` (`.HitActor` (`GameplayStatics.BreakHitResult` _array_element))))
    (`KismetSystemLibrary.DrawDebugSphere` _returnvalue (`KismetMathLibrary.VSize` (- _returnvalue _returnvalue_2)) 20 (struct :`R` 1.0 :`A` 1.0) 10.0 1.0)))

(event `self.ReceiveTick`
  (params (DeltaSeconds :type "Float (single-precision)")))

(fn `FindNearestPoint`
  (params (AnchorPoint :type "Array of Actor Object Reference") (ActorLocation :type "Vector Structure"))
  (returns (ActorRotation :type "Rotator Structure"))
  (for (_array_element _array_index) AnchorPoint
    (if (== _array_index 0)
      (bind _returnvalue (`KismetMathLibrary.VSize` (- (`self.K2_GetActorLocation` _array_element) ActorLocation)))
      (set `self.minDistance` _returnvalue)
      (set `self.NearestAnchorPoint` _array_element)
      (else
        (`/Engine/EditorBlueprintResources/StandardMacros.CompareFloat` (`self.minDistance`) _returnvalue
          (:`>`
            (set `self.minDistance` _returnvalue)
            (bind _output_get (set `self.NearestAnchorPoint` _array_element)))))))
  (`KismetSystemLibrary.PrintString` (`KismetSystemLibrary.GetDisplayName` _output_get))
  (return (`KismetMathLibrary.FindLookAtRotation` ActorLocation (`self.K2_GetActorLocation` (`self.NearestAnchorPoint`)))))

(fn `UserConstructionScript`)