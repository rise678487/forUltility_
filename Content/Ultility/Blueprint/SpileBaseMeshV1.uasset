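; A spline-driven placement utility actor that puts an instanced static mesh at each spline point, built entirely in the construction script.
; An array is nudged toward the spline point count by one entry per run, then drives the loop that adds instances.
; Each instance takes its point's local location and scale, with an optional flag to follow the spline's rotation.
; All instances share one configurable mesh.
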(fn `UserConstructionScript`
  (locals (`Góc quay của đối tượng cục bộ` :type "Rotator Structure"))
  (bind `_mảnh_chứa_tất_cả_đối_tượng` (`self.Mảnh chứa tất cả đối tượng`))
  (bind `_loại_mesh_mà_đối_tượng_hiển_thị` (`self.Loại Mesh mà đối tượng hiển thị`))
  (bind `_mảnh_chứa_tất_cả_đối_tượng_2` (`self.Mảnh chứa tất cả đối tượng`))
  (bind _instancedstaticmesh (`self.InstancedStaticMesh`))
  (bind _spline (`self.Spline`))
  (`|ExecutionSequence`
    (:`then_0`
      (set `self.Tổng Số Đối Tượng Hiện Có` (`SplineComponent.GetNumberOfSplinePoints` (`self.Spline`))))
    (:`then_1`
      (`/Engine/EditorBlueprintResources/StandardMacros.CompareInt` (`KismetArrayLibrary.Array_Length` `_mảnh_chứa_tất_cả_đối_tượng`) (`self.Tổng Số Đối Tượng Hiện Có`)
        (:`>`
          (`KismetArrayLibrary.Array_Remove` `_mảnh_chứa_tất_cả_đối_tượng_2` (`KismetArrayLibrary.Array_LastIndex` `_mảnh_chứa_tất_cả_đối_tượng_2`)))
        (:`<`
          (`KismetArrayLibrary.Array_Add` (`self.Mảnh chứa tất cả đối tượng`) `_loại_mesh_mà_đối_tượng_hiển_thị`))))
    (:`then_2`
      (for (_ _array_index) `_mảnh_chứa_tất_cả_đối_tượng`
        (`StaticMeshComponent.SetStaticMesh` _instancedstaticmesh (`.StaticMesh_2_5635248E41AFE4B0D5E64CAD1D506F8F` (break `/Game/Ultility/DataStructure/PointData` `_loại_mesh_mà_đối_tượng_hiển_thị`)))
        (if (`self.Bị ảnh hưởng bởi các góc quay của các đối tượng bên  cạnh`)
          (set `local.Góc quay của đối tượng cục bộ` (`SplineComponent.GetRotationAtSplinePoint` _spline _array_index "Local"))
          (else
            (set `local.Góc quay của đối tượng cục bộ` (struct))))
        (`InstancedStaticMeshComponent.AddInstance` _instancedstaticmesh (`KismetMathLibrary.MakeTransform` (`SplineComponent.GetLocationAtSplinePoint` _spline _array_index "Local") (`local.Góc quay của đối tượng cục bộ`) (`SplineComponent.GetScaleAtSplinePoint` _spline _array_index)))))))