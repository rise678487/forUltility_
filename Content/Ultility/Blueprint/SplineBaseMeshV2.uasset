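; Spline placement tool that scatters instanced static meshes along a spline onto the surface below.
; The construction script steps by spacing, applies optional random scale and offset, then line-traces down for each location.
; Instances follow spline rotation, get yaw from one or several anchor actors, or use optional random yaw.
; A random chance thins placement except with multiple anchors, where FindNearestAnchorPoint supplies yaw pointing away from the chosen anchor.
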(fn `FindNearestAnchorPoint`
  (params (AnchorArrays :type "Array of Actor Object Reference") (Location :type "Vector Structure"))
  (returns (OutputRotation :type "Rotator Structure") (`Nearest Anchor Point Location` :type "Vector Structure"))
  (locals (currentAchorPoint :type "Actor Object Reference") (minDistance :type "Float (double-precision)") (NearestAnchorPoint :type "Actor Object Reference"))
  (bind _returnvalue (`self.K2_GetActorLocation` (`local.NearestAnchorPoint`)))
  (if (> (`KismetArrayLibrary.Array_Length` AnchorArrays) 0)
    (for (_array_element _array_index) AnchorArrays
      (if (`KismetSystemLibrary.IsValid` _array_element)
        (if (== _array_index 0)
          (bind _returnvalue_2 (`KismetMathLibrary.VSize` (- (`self.K2_GetActorLocation` _array_element) Location)))
          (set `local.minDistance` _returnvalue_2)
          (else
            (`/Engine/EditorBlueprintResources/StandardMacros.CompareFloat` (`local.minDistance`) _returnvalue_2
              (:`>`
                (set `local.minDistance` _returnvalue_2)
                (set `local.NearestAnchorPoint` _array_element)))))))
    (return (`KismetMathLibrary.FindLookAtRotation` _returnvalue Location) _returnvalue)))

(fn `UserConstructionScript`
  (bind `_loại_mesh_muốn_thêm_staticmesh` (break `/Game/Ultility/DataStructure/PointData` (`self.Loại Mesh muốn thêm`)))
  (bind _anchor_point (`self.Anchor Point`))
  (bind `_khoảng_cách_xê_dịch` (`self.Khoảng cách xê dịch`))
  (bind `_kích_thước_của_đối_tượng` (`self.Kích thước của đối tượng`))
  (bind `_khoảng_cách_giữa_các_đối_tượng` (`self.Khoảng cách giữa các đối tượng`))
  (bind _spline (`self.Spline`))
  (bind `_góc_quay_được_tạo_ngẫu_nhiên` (`self.Góc quay được tạo ngẫu nhiên`))
  (bind `_kích_thước_của_đối_tượng_2` (`self.Kích thước của đối tượng`))
  (bind `_kích_thước_của_đối_tượng_3` (`self.Kích thước của đối tượng`))
  (bind `_kích_thước_của_đối_tượng_4` (`self.Kích thước của đối tượng`))
  (bind _returnvalue (`self.K2_GetActorLocation` _anchor_point))
  (if (`self.refresh`)
    _
    (else
      _))
  (set `self.refresh` false)
  (`StaticMeshComponent.SetStaticMesh` (`self.InstancedStaticMesh`) `_loại_mesh_muốn_thêm_staticmesh`)
  (for _index (range (+ (`.ReturnValue` (`KismetMathLibrary.FMod` (`SplineComponent.GetSplineLength` _spline) `_khoảng_cách_giữa_các_đối_tượng`)) 1))
    ;[1 1 1] Tạo kích thước ngẫu nhiên
    (if (`self.Có sử dụng kích thước ngẫu nhiên`)
      (set `self.Kích thước của đối tượng` (`KismetMathLibrary.RandomFloatInRange` (`self.Kích thước nhỏ nhất`) (`self.Kích thước lớn nhất`)))
      (else
        (set `self.Kích thước của đối tượng` 1.0)))
    ;[1 1 1] Tạo Góc quay ngẫu nhiên
    (if (`self.Có sử dụng góc quay ngẫu nhiên`)
      (set `self.Góc quay của đối tượng` (`KismetMathLibrary.RandomFloatInRange` (* `_góc_quay_được_tạo_ngẫu_nhiên` -1.0) `_góc_quay_được_tạo_ngẫu_nhiên`))
      (else
        (set `self.Góc quay của đối tượng` 0.0)))
    ;[1 1 1] Tạo vị trí ngẫu nhiên trái phải
    (if (`self.Sử dụng vị trí 2 bên ngẫu nhiên`)
      (set `self.Khoảng cách xê dịch` (`KismetMathLibrary.RandomFloatInRange` (* (`self.Khoảng cách xê dịch bên trái`) -1.0) (`self.Khoảng cách xê dịch bên phải`)))
      (else
        (set `self.Khoảng cách xê dịch` 0.0)))
    (bind _returnvalue_2 (* _index `_khoảng_cách_giữa_các_đối_tượng`))
    (bind (_returnvalue_x _returnvalue_y _returnvalue_z) (`KismetMathLibrary.BreakVector` (`SplineComponent.GetLocationAtDistanceAlongSpline` _spline _returnvalue_2 "World")))
    (bind _x (.x (`KismetMathLibrary.MakeVector` (+ _returnvalue_x `_khoảng_cách_xê_dịch`) (+ _returnvalue_y `_khoảng_cách_xê_dịch`) (+ (`self.Chiều cao lớn nhất của địa hình`) _returnvalue_z))))
    (bind _y (.y (`KismetMathLibrary.MakeVector` (+ _returnvalue_x `_khoảng_cách_xê_dịch`) (+ _returnvalue_y `_khoảng_cách_xê_dịch`) (+ (`self.Chiều cao lớn nhất của địa hình`) _returnvalue_z))))
    (bind _outhit (`KismetSystemLibrary.LineTraceSingle` :`Start` (`KismetMathLibrary.MakeVector` _x _y (.z (`KismetMathLibrary.MakeVector` (+ _returnvalue_x `_khoảng_cách_xê_dịch`) (+ _returnvalue_y `_khoảng_cách_xê_dịch`) (+ (`self.Chiều cao lớn nhất của địa hình`) _returnvalue_z)))) :`End` (`KismetMathLibrary.MakeVector` _x _y -1000.0) :`TraceChannel` "TraceTypeQuery1" :`bTraceComplex` true :`DrawDebugType` "ForDuration"))
    (if (`self.xoay theo đường dẫn`)
      ;[1 1 1] Xoay theo Spline
      (if (< (`KismetMathLibrary.RandomIntegerInRange` 0 10) (`self.tỷ lệ diễn ra random`))
        (`InstancedStaticMeshComponent.AddInstanceWorldSpace` (`self.InstancedStaticMesh`) (`KismetMathLibrary.MakeTransform` (`.Location` (`GameplayStatics.BreakHitResult` _outhit)) (`SplineComponent.GetRotationAtDistanceAlongSpline` _spline _returnvalue_2 "World") (`KismetMathLibrary.MakeVector` `_kích_thước_của_đối_tượng_3` `_kích_thước_của_đối_tượng_3` `_kích_thước_của_đối_tượng_3`))))
      (elif (`self.Xoay theo 1 điểm`)
        ;[1 1 1] Anchor Point
        (if (`KismetSystemLibrary.IsValid` _anchor_point)
          (set `self.xoay theo đường dẫn` false)
          (set `self.Có sử dụng góc quay ngẫu nhiên` false)
          (if (< (`KismetMathLibrary.RandomIntegerInRange` 0 10) (`self.tỷ lệ diễn ra random`))
            (`KismetSystemLibrary.DrawDebugLine` (`.Location` (`GameplayStatics.BreakHitResult` _outhit)) _returnvalue (struct :`R` 1.0 :`A` 1.0) 50.0 1.0)
            (bind (_returnvalue_roll _returnvalue_pitch _returnvalue_yaw) (`KismetMathLibrary.BreakRotator` (`KismetMathLibrary.FindLookAtRotation` (`.Location` (`GameplayStatics.BreakHitResult` _outhit)) _returnvalue)))
            (`InstancedStaticMeshComponent.AddInstanceWorldSpace` (`self.InstancedStaticMesh`) (`KismetMathLibrary.MakeTransform` (`.Location` (`GameplayStatics.BreakHitResult` _outhit)) (`KismetMathLibrary.MakeRotator` 0.0 0.0 _returnvalue_yaw) (`KismetMathLibrary.MakeVector` `_kích_thước_của_đối_tượng` `_kích_thước_của_đối_tượng` `_kích_thước_của_đối_tượng`))))
          (elif (`self.Sử dụng nhiều anchor point`)
            (bind (_outputrotation _nearest_anchor_point_location) (`self.FindNearestAnchorPoint` (`self.AnchorPoints`) (`.Location` (`GameplayStatics.BreakHitResult` _outhit))))
            (`KismetSystemLibrary.DrawDebugLine` (`.Location` (`GameplayStatics.BreakHitResult` _outhit)) _nearest_anchor_point_location (struct :`R` 1.0 :`A` 1.0) 50.0 1.0)
            (`InstancedStaticMeshComponent.AddInstanceWorldSpace` (`self.InstancedStaticMesh`) (`KismetMathLibrary.MakeTransform` (`.Location` (`GameplayStatics.BreakHitResult` _outhit)) (`KismetMathLibrary.MakeRotator` 0.0 0.0 (.yaw _outputrotation)) (`KismetMathLibrary.MakeVector` `_kích_thước_của_đối_tượng_2` `_kích_thước_của_đối_tượng_2` `_kích_thước_của_đối_tượng_2`)))))
        (else
          ;[1 1 1] Random Rotation
          (if (< (`KismetMathLibrary.RandomIntegerInRange` 0 10) (`self.tỷ lệ diễn ra random`))
            (`InstancedStaticMeshComponent.AddInstanceWorldSpace` (`self.InstancedStaticMesh`) (`KismetMathLibrary.MakeTransform` (`.Location` (`GameplayStatics.BreakHitResult` _outhit)) (`KismetMathLibrary.MakeRotator` 0.0 0.0 (`self.Góc quay của đối tượng`)) (`KismetMathLibrary.MakeVector` `_kích_thước_của_đối_tượng_4` `_kích_thước_của_đối_tượng_4` `_kích_thước_của_đối_tượng_4`)))))))))